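; BP_Lift is a lift actor for Level 3 that moves toward an end position while its trigger is overlapped and back toward its start when the overlap ends.
; Overlap begin and end switch the target position and play or reverse a timeline, with no filter on the overlapping actor.
; Each update lerps from the current location, not a fixed origin, so reversing applies a falling alpha toward the start.
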(event `self.ReceiveBeginPlay`
  (set `self.StartPos` (`self.K2_GetActorLocation`)))

(event `self.Trigger.OnComponentBeginOverlap`
  (params (OverlappedComponent :type "PrimitiveComponent Object Reference") (OtherActor :type "Actor Object Reference") (OtherComp :type "PrimitiveComponent Object Reference") (OtherBodyIndex :type Integer) (bFromSweep :type Boolean) (SweepResult :type "HitResult Structure (by ref)"))
  (set `self.MoveToPos` (`self.EndPos`))
  (bind (_direction _newtrack_0) (`Timeline|LiftTimeline` :!label _label)
    (:`Update`
      (`self.K2_SetActorLocation` (`KismetMathLibrary.VLerp` (`self.K2_GetActorLocation`) (`self.MoveToPos`) _newtrack_0)))))

(event `self.Trigger.OnComponentEndOverlap`
  (params (OverlappedComponent :type "PrimitiveComponent Object Reference") (OtherActor :type "Actor Object Reference") (OtherComp :type "PrimitiveComponent Object Reference") (OtherBodyIndex :type Integer))
  (set `self.MoveToPos` (`self.StartPos`))
  (goto _label :!via `Reverse`))

(fn `UserConstructionScript`)