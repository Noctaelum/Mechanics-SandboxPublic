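; BP_Ladder is a ladder actor for level 4 that tells player characters when they are in its overlap area.
; On begin overlap it sets IsOnLadder on either a FirstPersonCharacter or a CustomFPCharacter, handling each class on its own Sequence branch.
; On end overlap it clears the flag and resets that character's movement mode to Walking.
; It does no climbing movement itself.
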(event `self.ReceiveActorBeginOverlap`
  (params (OtherActor :type "Actor Object Reference"))
  (`|ExecutionSequence`
    (:`then_0`
      (bind _asfirst_person_character (cast `/Game/FirstPersonBP/Blueprints/FirstPersonCharacter` OtherActor))
      (set `/Game/FirstPersonBP/Blueprints/FirstPersonCharacter.IsOnLadder` true _asfirst_person_character))
    (:`then_1`
      (bind _ascustom_fpcharacter (cast `CustomFPCharacter` OtherActor))
      (set `CustomFPCharacter.IsOnLadder` true _ascustom_fpcharacter))))

(event `self.ReceiveActorEndOverlap`
  (params (OtherActor :type "Actor Object Reference"))
  (`|ExecutionSequence`
    (:`then_0`
      (bind _asfirst_person_character (cast `/Game/FirstPersonBP/Blueprints/FirstPersonCharacter` OtherActor))
      (set `/Game/FirstPersonBP/Blueprints/FirstPersonCharacter.IsOnLadder` false _asfirst_person_character)
      (`CharacterMovementComponent.SetMovementMode` (`Character.CharacterMovement` _asfirst_person_character) "MOVE_Walking" 0))
    (:`then_1`
      (bind _ascustom_fpcharacter (cast `CustomFPCharacter` OtherActor))
      (set `CustomFPCharacter.IsOnLadder` false _ascustom_fpcharacter)
      (`CharacterMovementComponent.SetMovementMode` (`Character.CharacterMovement` _ascustom_fpcharacter) "MOVE_Walking" 0))))

(fn `UserConstructionScript`)